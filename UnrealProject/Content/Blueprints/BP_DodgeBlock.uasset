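; BP_DodgeBlock is a moving obstacle that the VR player dodges.
; Each tick it moves along BlockMoveDirection at BlockSpeed, without sweep, and destroys itself once its X position passes a fixed threshold.
; Mesh overlap with the VRPawn decrements Lives and calls UpdateLives.
; A separate Box overlap plays a level-up sound and calls UpdateLives with -1, leaving Lives untouched in this Blueprint.
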(event OnComponentBeginOverlap(Box)
  (params (OverlappedComponent :type Primitive%20Component%20Object%20Reference) (OtherActor :type Actor%20Object%20Reference) (OtherComp :type Primitive%20Component%20Object%20Reference) (OtherBodyIndex :type Integer) (bFromSweep :type Boolean) (SweepResult :type Hit%20Result%20Structure%20%28by%20ref%29))
  (bind _asvrpawn (Utilities|Casting|CastToVRPawn OtherActor))
  (Audio|PlaySound2D "/Game/439889__simonbay__lushlife_levelup.439889__simonbay__lushlife_levelup" 1.0 1.0 0.0 0 0)
  (Default|UpdateLives _asvrpawn -1))

(event OnComponentBeginOverlap(StaticMesh)
  (params (OverlappedComponent :type Primitive%20Component%20Object%20Reference) (OtherActor :type Actor%20Object%20Reference) (OtherComp :type Primitive%20Component%20Object%20Reference) (OtherBodyIndex :type Integer) (bFromSweep :type Boolean) (SweepResult :type Hit%20Result%20Structure%20%28by%20ref%29))
  (bind _asvrpawn (Utilities|Casting|CastToVRPawn OtherActor))
  (Variables|/Game/VRTemplate/Blueprints/VRPawn.VRPawn_C|SetLives _asvrpawn (- (Variables|/Game/VRTemplate/Blueprints/VRPawn.VRPawn_C|GetLives _asvrpawn) 1))
  (Default|UpdateLives _asvrpawn))

(event EventBeginPlay)

(event Collision|EventActorBeginOverlap
  (params (OtherActor :type Actor%20Object%20Reference)))

(event EventTick
  (params (DeltaSeconds :type Float%20%28single-precision%29))
  (Transformation|SetActorLocation (+ (* (Variables|Default|GetBlockMoveDirection) (* (Variables|Default|GetBlockSpeed) DeltaSeconds)) (Transformation|GetActorLocation)) false false)
  (if (> (.X (Math|Vector|BreakVector (Transformation|GetActorLocation))) -2.5e+02)
    (Actor|DestroyActor)))

(fn ConstructionScript)