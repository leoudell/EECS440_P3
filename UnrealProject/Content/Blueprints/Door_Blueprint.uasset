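; Door Blueprint that slides an actor open or closed by adding a world offset every Tick while ShouldOpen or ShouldClose is set.
; A one-second Delay ends each movement by clearing its flag and updating IsOpen, so travel distance depends on frame rate.
; SetIsOpen and SetIsMoving both only toggle ShouldOpen, and nothing here sets ShouldClose to true.
; OpenRight is empty and GetIsMoving always returns false.
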(event EventBeginPlay)

(event Collision|EventActorBeginOverlap
  (params (OtherActor :type Actor%20Object%20Reference)))

(event EventTick
  (params (DeltaSeconds :type Float%20%28single-precision%29))
  (if (Variables|Default|GetShouldOpen)
    (Transformation|AddActorWorldOffset (Variables|Default|GetMovement))
    (Utilities|FlowControl|Delay 1.0)
    (Variables|Default|SetShouldOpen false)
    (Variables|Default|SetIsOpen true)
    (elif (Variables|Default|GetShouldClose)
      (Transformation|AddActorWorldOffset (Variables|Default|GetNegativeMovement))
      (Utilities|FlowControl|Delay 1.0)
      (Variables|Default|SetShouldClose false)
      (Variables|Default|SetIsOpen false))))

(fn ConstructionScript)

(fn OpenRight)

(fn SetIsOpen
  (Variables|Default|SetShouldOpen (not (Variables|Default|GetShouldOpen))))

(fn SetIsMoving
  (Variables|Default|SetShouldOpen (not (Variables|Default|GetShouldOpen))))

(fn GetIsMoving
  (return false))