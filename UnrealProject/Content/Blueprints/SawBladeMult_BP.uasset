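; Moving saw-blade obstacle with several blades that costs the VR player a life on contact.
; BeginPlay removes one of four blade meshes at random to leave a gap, then spawns an attached heart above it (the chance check always passes).
; Tick moves the actor along its block direction and speed.
; Blade overlap with VRPawn plays a grunt, deducts a life, destroys obstacle and heart, and fades the camera to white.
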(event OnComponentBeginOverlap(StaticMesh1)
  (params (OverlappedComponent :type Primitive%20Component%20Object%20Reference) (OtherActor :type Actor%20Object%20Reference) (OtherComp :type Primitive%20Component%20Object%20Reference) (OtherBodyIndex :type Integer) (bFromSweep :type Boolean) (SweepResult :type Hit%20Result%20Structure%20%28by%20ref%29))
  (CallFunction|Collision OtherActor))

(event OnComponentBeginOverlap(StaticMesh4)
  (params (OverlappedComponent :type Primitive%20Component%20Object%20Reference) (OtherActor :type Actor%20Object%20Reference) (OtherComp :type Primitive%20Component%20Object%20Reference) (OtherBodyIndex :type Integer) (bFromSweep :type Boolean) (SweepResult :type Hit%20Result%20Structure%20%28by%20ref%29))
  (CallFunction|Collision OtherActor))

(event OnComponentBeginOverlap(StaticMesh7)
  (params (OverlappedComponent :type Primitive%20Component%20Object%20Reference) (OtherActor :type Actor%20Object%20Reference) (OtherComp :type Primitive%20Component%20Object%20Reference) (OtherBodyIndex :type Integer) (bFromSweep :type Boolean) (SweepResult :type Hit%20Result%20Structure%20%28by%20ref%29))
  (CallFunction|Collision OtherActor))

(event OnComponentBeginOverlap(StaticMesh12)
  (params (OverlappedComponent :type Primitive%20Component%20Object%20Reference) (OtherActor :type Actor%20Object%20Reference) (OtherComp :type Primitive%20Component%20Object%20Reference) (OtherBodyIndex :type Integer) (bFromSweep :type Boolean) (SweepResult :type Hit%20Result%20Structure%20%28by%20ref%29))
  (CallFunction|Collision OtherActor))

(event EventBeginPlay
  (bind _output_get (Variables|Default|SetHiddenIndex (Math|Random|RandomIntegerinRange 0 3)))
  (Variables|Default|SetHeartLoc (Math|Vector|MakeVector (.x (Transformation|GetWorldLocation (Utilities|Array|Get(acopy) (Utilities|Array|MakeArray (Variables|Default|GetStaticMesh1) (Variables|Default|GetStaticMesh4) (Variables|Default|GetStaticMesh7) (Variables|Default|GetStaticMesh12)) _output_get))) (.y (Transformation|GetWorldLocation (Utilities|Array|Get(acopy) (Utilities|Array|MakeArray (Variables|Default|GetStaticMesh1) (Variables|Default|GetStaticMesh4) (Variables|Default|GetStaticMesh7) (Variables|Default|GetStaticMesh12)) _output_get))) (+ (.z (Transformation|GetWorldLocation (Utilities|Array|Get(acopy) (Utilities|Array|MakeArray (Variables|Default|GetStaticMesh1) (Variables|Default|GetStaticMesh4) (Variables|Default|GetStaticMesh7) (Variables|Default|GetStaticMesh12)) _output_get))) 3.5e+02)))
  (Components|DestroyComponent (Utilities|Array|Get(acopy) (Utilities|Array|MakeArray (Variables|Default|GetStaticMesh1) (Variables|Default|GetStaticMesh4) (Variables|Default|GetStaticMesh7) (Variables|Default|GetStaticMesh12)) _output_get))
  (Utilities|FlowControl|Delay 1.0)
  (if (<= (Math|Random|RandomFloatinRange 0.0 1.0) 1.0)
    (bind _returnvalue (Game|SpawnActorfromClass "/Game/Blueprints/BP_Heart.BP_Heart_C" (Math|Transform|MakeTransform "0, 0, 0" "0, 0, 0" "1.000000,1.000000,1.000000") "AlwaysSpawn" "MultiplyWithRoot" 0 0))
    (bind _output_get_2 (Variables|Default|SetHeartActor _returnvalue))
    (Transformation|AttachComponentToComponent _output_get_2 (Variables|Default|GetDefaultSceneRoot) "None" "SnapToTarget" "KeepRelative" "KeepRelative" true)
    (Transformation|SetActorTransform (Variables|Default|GetHeartActor) (Math|Transform|MakeTransform (Variables|Default|GetHeartLoc) "0, 0, 0" "1.000000,1.000000,1.000000"))
    (Variables|/Game/Blueprints/BP_Heart.BP_Heart_C|SetAttached (Variables|Default|GetHeartActor) true)
    (Actor|Tick|SetActorTickEnabled true)
    (else
      (Actor|Tick|SetActorTickEnabled true))))

(event EventTick
  (params (DeltaSeconds :type Float%20%28single-precision%29))
  (Transformation|SetActorLocation (+ (* (Variables|Default|GetBlockMoveDirection) (* (Variables|Default|GetBlockSpeed) DeltaSeconds)) (Transformation|GetActorLocation)) false false))

(fn ConstructionScript)

(fn Collision
  (params (OtherActor :type Actor%20Object%20Reference))
  (bind _asvrpawn (Utilities|Casting|CastToVRPawn OtherActor))
  (Audio|PlaySound2D "/Game/Audio/497713__miksmusic__punch-grunt-1.497713__miksmusic__punch-grunt-1" 1.0 1.0 0.0 0 0)
  (Default|UpdateLives _asvrpawn -1)
  (Actor|DestroyActor)
  (Actor|DestroyActor (Variables|Default|GetHeartActor))
  (Actor|Tick|SetActorTickEnabled false)
  (CameraFades|StartCameraFade (Variables|/Script/Engine.PlayerController|GetPlayerCameraManager (Game|GetPlayerController 0)) 0.0 1.0 0.1 "(R=1.000000,G=1.000000,B=1.000000,A=1.000000)" false false))