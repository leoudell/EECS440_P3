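; Laser projectile actor for a VR game that costs the VRPawn one life when its mesh begins overlapping it.
; On BeginPlay it faces the player and sets its movement along the player-to-laser axis, scaled by Speed.
; Tick offsets it by that vector without sweep or delta-time scaling.
; A Deflect event reflects the vector off a supplied surface normal, leaving the actor's rotation unchanged.
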(event OnComponentBeginOverlap(StaticMesh)
  (params (OverlappedComponent :type Primitive%20Component%20Object%20Reference) (OtherActor :type Actor%20Object%20Reference) (OtherComp :type Primitive%20Component%20Object%20Reference) (OtherBodyIndex :type Integer) (bFromSweep :type Boolean) (SweepResult :type Hit%20Result%20Structure%20%28by%20ref%29))
  (bind _asvrpawn (Utilities|Casting|CastToVRPawn OtherActor))
  (Default|UpdateLives _asvrpawn -1))

(event Custom|Deflect
  (params (NewParam :type Vector))
  (Variables|Default|SetMovementDirection (Math|Vector|GetReflectionVector (Variables|Default|GetMovementDirection) NewParam)))

(event Collision|EventActorBeginOverlap
  (params (OtherActor :type Actor%20Object%20Reference)))

(event EventBeginPlay
  (Transformation|SetActorRotation (Math|Rotator|FindLookatRotation (Transformation|GetActorLocation) (Transformation|GetActorLocation (Game|Player|GetPlayerPawn 0))))
  (Variables|Default|SetMovementDirection (* (Math|Vector|Normalize (- (Transformation|GetActorLocation) (Transformation|GetActorLocation (Game|Player|GetPlayerPawn 0)))) (Variables|Default|GetSpeed))))

(event EventTick
  (params (DeltaSeconds :type Float%20%28single-precision%29))
  (Transformation|AddActorWorldOffset (Variables|Default|GetMovementDirection)))

(fn ConstructionScript)