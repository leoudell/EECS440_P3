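; Console actor that runs a timed VR minigame, spawning obstacles while the referenced AffDoorSaw reports the game has started.
; A looping timer set on BeginPlay drives delayed spawns of blocks, or occasionally UFOs, at fixed locations.
; Tick counts down the game timer on the VRPawn's text display.
; At zero it clears the spawn timer, hides the text and enables teleporting.
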(event Custom|Spawn%20Block
  (if (Variables|/Game/Affordances/AffDoorSaw.AffDoorSaw_C|GetGameStarted (Variables|Default|GetAffDoorSaw))
    (Utilities|FlowControl|Delay 2.0)
    (bind _asvrpawn (Utilities|Casting|CastToVRPawn (Game|Player|GetPlayerPawn 0)))
    (Rendering|SetVisibility (Variables|/Game/VRTemplate/Blueprints/VRPawn.VRPawn_C|GetTimerText _asvrpawn) true false)
    (if (<= (Math|Random|RandomFloatinRange 0.0 1.0) 0.2)
      (Game|SpawnActorfromClass (Variables|Default|GetUFOClass) (Math|Transform|MakeTransform (Math|Vector|MakeVector -2e+03 1.2e+02 2.5e+02) "0, 0, 0" "1.000000,1.000000,1.000000") "AlwaysSpawn" "MultiplyWithRoot" 0 0)
      (else
        (Game|SpawnActorfromClass (Variables|Default|GetBlockClass) (Math|Transform|MakeTransform (Math|Vector|MakeVector -2e+03 1.2e+02 8e+01) "0.000000,90.000000,0.000000" "1.000000,1.000000,1.000000") "AlwaysSpawn" "MultiplyWithRoot" 0 0)))
    (else
      (Development|PrintText "Not Open"))))

(event EventBeginPlay
  (bind _returnvalue (Utilities|Time|SetTimerbyEvent (EventDispatchers|CreateEvent :!event Custom|Spawn%20Block) (Variables|Default|GetSpawnInterval) true))
  (Variables|Default|SetSpawnerHandle _returnvalue))

(event EventTick
  (params (DeltaSeconds :type Float%20%28single-precision%29))
  (if (Variables|/Game/Affordances/AffDoorSaw.AffDoorSaw_C|GetGameStarted (Variables|Default|GetAffDoorSaw))
    (bind _output_get (Variables|Default|SetGameTimer (- (Variables|Default|GetGameTimer) DeltaSeconds)))
    (bind _asvrpawn (Utilities|Casting|CastToVRPawn (Game|Player|GetPlayerPawn 0)))
    (Rendering|Components|TextRender|SetText (Variables|/Game/VRTemplate/Blueprints/VRPawn.VRPawn_C|GetTimerText _asvrpawn) (Utilities|Text|ToText(String) (Class|KismetMathLibrary|Round64 _output_get)))
    (if (<= _output_get 0.0)
      (Utilities|Time|ClearandInvalidateTimerbyHandle (Variables|Default|GetSpawnerHandle))
      (Rendering|SetVisibility (Variables|/Game/VRTemplate/Blueprints/VRPawn.VRPawn_C|GetTimerText _asvrpawn) false false)
      (Variables|/Game/VRTemplate/Blueprints/VRPawn.VRPawn_C|SetTeleportEnabled _asvrpawn true))))

(fn ConstructionScript)