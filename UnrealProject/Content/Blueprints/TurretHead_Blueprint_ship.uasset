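; Ship turret head that fires lasers once Attack_ship starts it and re-enables VR teleporting when destroyed.
; Tick updates a lives text, occasionally yaws a mesh toward the player with random offset, and spawns lasers from its arrow after random delays.
; Box overlaps each remove a life and play a sound, destroying the turret at zero.
; BeginPlay also sets a looping timer and opens a gate if the door's ShouldOpen is set.
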(event OnComponentBeginOverlap(Box)
  (params (OverlappedComponent :type Primitive%20Component%20Object%20Reference) (OtherActor :type Actor%20Object%20Reference) (OtherComp :type Primitive%20Component%20Object%20Reference) (OtherBodyIndex :type Integer) (bFromSweep :type Boolean) (SweepResult :type Hit%20Result%20Structure%20%28by%20ref%29))
  (bind _returnvalue (Transformation|GetActorLocation))
  (bind _output_get (Variables|Default|SetTurretLives (- (Variables|Default|GetTurretLives) 1)))
  (if (== _output_get 0)
    (Actor|DestroyActor)
    (Audio|PlaySoundatLocation "/Game/Audio/87040__runnerpack__stun.87040__runnerpack__stun" _returnvalue "0, 0, 0" 1.0 1.0 0.0 0 0 0 0)
    (bind _asvrpawn (Utilities|Casting|CastToVRPawn (Game|Player|GetPlayerPawn 0)))
    (Variables|/Game/VRTemplate/Blueprints/VRPawn.VRPawn_C|SetTeleportEnabled _asvrpawn true)
    (else
      (Audio|PlaySoundatLocation "/Game/Audio/459150__lilmati__retro-underwater-explosion.459150__lilmati__retro-underwater-explosion" _returnvalue "0, 0, 0" 1.0 1.0 0.0 0 0 0 0))))

(event Custom|Fire
  (Utilities|FlowControl|Gate true))

(event Custom|Attack_ship
  (Variables|Default|Setstarted true))

(event EventBeginPlay
  (Utilities|Time|SetTimerbyEvent (EventDispatchers|CreateEvent :!event Custom|Fire) 1.5 true)
  (bind _returnvalue (Actor|GetActorOfClass "/Game/Blueprints/Door_Blueprint.Door_Blueprint_C"))
  (if (Variables|/Game/Blueprints/Door_Blueprint.Door_Blueprint_C|GetShouldOpen _returnvalue)
    (Utilities|FlowControl|Gate true) ; enters at Open
  ))

(event EventTick
  (params (DeltaSeconds :type Float%20%28single-precision%29))
  (bind _returnvalue (Actor|GetComponentbyClass "/Script/Engine.ArrowComponent"))
  (bind _returnvalue_2 (Transformation|GetWorldTransform _returnvalue))
  (bind (_location _rotation _scale) (Math|Transform|BreakTransform _returnvalue_2))
  (Rendering|Components|TextRender|SetText (Variables|Default|GetTextRender) (Utilities|Text|FormatText "Lives: {TurretLives}" (Utilities|Text|ToText(Integer) (Variables|Default|GetTurretLives))))
  (if (== (Math|Float|%(Float) DeltaSeconds 5.0) 0.0)
    (Transformation|SetWorldRotation (Variables|Default|GetStaticMeshActor_28) (Math|Rotator|MakeRotator 0.0 0.0 (+ (+ (.yaw (Math|Rotator|FindLookatRotation (Transformation|GetActorLocation) (Transformation|GetActorLocation (Game|Player|GetPlayerPawn 0)))) (Math|Random|RandomFloatinRange 0.0 1e+01)) -9e+01)) false false))
  (Utilities|FlowControl|Delay (Math|Random|RandomFloatinRange 2.0 5.0))
  (if (Variables|Default|Getstarted)
    (Game|SpawnActorfromClass "/Game/Blueprints/Laser_Blueprint.Laser_Blueprint_C" (Math|Transform|MakeTransform _location _rotation _scale) "Undefined" "MultiplyWithRoot" 0 0)))

(fn ConstructionScript)