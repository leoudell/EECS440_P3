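; BP_CutoutWall_Crouch is a moving wall obstacle with a TopSection hit volume, named for crouching under in VR.
; On BeginPlay, a timeline lerps it a fixed distance along world +X without sweeping, then destroys it when finished.
; The first TopSection overlap by a VRPawn sets the HasHitPlayer flag, with no further response in this graph.
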(event OnComponentBeginOverlap(TopSection)
  (params (OverlappedComponent :type Primitive%20Component%20Object%20Reference) (OtherActor :type Actor%20Object%20Reference) (OtherComp :type Primitive%20Component%20Object%20Reference) (OtherBodyIndex :type Integer) (bFromSweep :type Boolean) (SweepResult :type Hit%20Result%20Structure%20%28by%20ref%29))
  (Utilities|Casting|CastToVRPawn OtherActor)
  (if (not (Variables|Default|GetbHasHitPlayer))
    (Variables|Default|SetbHasHitPlayer true)))

(event EventBeginPlay
  (bind _output_get (Variables|Default|SetStartLocation (Transformation|GetActorLocation)))
  (Variables|Default|SetEndLocation (- _output_get "-1200.000000,0.000000,0.000000"))
  (bind _alpha (Timeline|MoveTimeline Play)
    (:Update
      (Transformation|SetActorLocation (Math|Vector|Lerp(Vector) (Variables|Default|GetStartLocation) (Variables|Default|GetEndLocation) _alpha) false false))
    (:Finished
      (Actor|DestroyActor))))

(event Collision|EventActorBeginOverlap
  (params (OtherActor :type Actor%20Object%20Reference)))

(event EventTick
  (params (DeltaSeconds :type Float%20%28single-precision%29)))

(fn ConstructionScript)