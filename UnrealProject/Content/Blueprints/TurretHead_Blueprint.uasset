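; Turret head Blueprint that turns to track the player pawn and spawns lasers.
; Each Tick sets the yaw of a child actor component and its actor's arrow from a look-at rotation with a fixed offset, and debug-prints the arrow's name.
; BeginPlay starts a looping timer, and Fire spawns Laser_Blueprint at its own arrow's location with a fixed rotation rather than the aim.
; An older aim-and-fire chain is left unconnected.
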(event Custom|Fire
  (bind _returnvalue (Actor|GetComponentbyClass "/Script/Engine.ArrowComponent"))
  (bind _returnvalue_2 (Transformation|GetWorldTransform _returnvalue))
  (bind (_location _rotation _scale) (Math|Transform|BreakTransform _returnvalue_2))
  (Game|SpawnActorfromClass "/Game/Blueprints/Laser_Blueprint.Laser_Blueprint_C" (Math|Transform|MakeTransform _location "90.000000,0.000000,0.000000" _scale) "Undefined" "MultiplyWithRoot" 0 0))

(event EventBeginPlay
  (Utilities|Time|SetTimerbyEvent (EventDispatchers|CreateEvent :!event Custom|Fire) 1.5 true))

(event Collision|EventActorBeginOverlap
  (params (OtherActor :type Actor%20Object%20Reference)))

(event EventTick
  (params (DeltaSeconds :type Float%20%28single-precision%29))
  (bind _returnvalue (Game|Player|GetPlayerPawn 0))
  (bind _staticmeshactor_28 (Variables|Default|GetStaticMeshActor_28))
  (bind _returnvalue_2 (Transformation|GetActorLocation _returnvalue))
  (bind _childactor (Variables|/Script/Engine.ChildActorComponent|GetChildActor _staticmeshactor_28))
  (bind _returnvalue_3 (Transformation|GetActorLocation _childactor))
  (bind _returnvalue_4 (Actor|GetComponentbyClass _childactor "/Script/Engine.ArrowComponent"))
  (bind _returnvalue_5 (Math|Rotator|FindLookatRotation _returnvalue_3 _returnvalue_2))
  (bind _yaw (Math|Rotator|BreakRotator _returnvalue_5))
  (bind _returnvalue_6 (+ _yaw -92.0))
  (Development|PrintString (Utilities|GetDisplayName _returnvalue_4))
  (Transformation|SetRelativeRotation _staticmeshactor_28 (Math|Rotator|MakeRotator 0.0 0.0 _returnvalue_6) false false)
  (Transformation|SetWorldRotation _returnvalue_4 (Math|Rotator|MakeRotator 0.0 0.0 _returnvalue_6) false false))

(fn ConstructionScript)