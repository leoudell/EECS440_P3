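; UFO hazard actor that flies in a straight line and damages the player's ship on contact.
; Tick moves it along BlockMoveDirection at BlockSpeed, scaled by delta time.
; When its Box overlaps a VRPawn, it plays an explosion sound, takes away a life and some ship health, destroys itself and triggers the pawn's ship explosion.
; A camera shake node is present but never runs.
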(event OnComponentBeginOverlap(Box)
  (params (OverlappedComponent :type Primitive%20Component%20Object%20Reference) (OtherActor :type Actor%20Object%20Reference) (OtherComp :type Primitive%20Component%20Object%20Reference) (OtherBodyIndex :type Integer) (bFromSweep :type Boolean) (SweepResult :type Hit%20Result%20Structure%20%28by%20ref%29))
  (bind _asvrpawn (Utilities|Casting|CastToVRPawn OtherActor))
  (Audio|PlaySound2D "/Game/Audio/446624__idkmrgarcia__explosion2.446624__idkmrgarcia__explosion2" 1.0 1.0 0.0 0 0)
  (Default|UpdateLives _asvrpawn -1)
  (Default|UpdateShipHealth _asvrpawn -0.1)
  (Actor|DestroyActor)
  (Default|ShipExplosion _asvrpawn))

(event EventBeginPlay)

(event Collision|EventActorBeginOverlap
  (params (OtherActor :type Actor%20Object%20Reference)))

(event EventTick
  (params (DeltaSeconds :type Float%20%28single-precision%29))
  (bind _returnvalue (Transformation|GetActorLocation))
  (bind _blockmovedirection (Variables|Default|GetBlockMoveDirection))
  (bind _blockspeed (Variables|Default|GetBlockSpeed))
  (bind _returnvalue_2 (* _blockspeed DeltaSeconds))
  (bind _returnvalue_3 (* _blockmovedirection _returnvalue_2))
  (bind _returnvalue_4 (+ _returnvalue_3 _returnvalue))
  (Transformation|SetActorLocation (Math|Vector|MakeVector (.x _returnvalue_4) (.y _returnvalue_4) (.z _returnvalue_4)) false false))

(fn ConstructionScript)